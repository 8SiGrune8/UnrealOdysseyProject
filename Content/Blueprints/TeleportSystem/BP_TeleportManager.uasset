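; BP_TeleportManager is a manager actor that moves the player character to a selected teleport target in the level.
; On BeginPlay it collects all BP_TeleportTarget actors and their names, then shows UI_TeleportMenu with a reference to itself.
; ExecuteTeleport plays a fade out on a UI_FadeOverlay, waits briefly, starts the fade in, then sets the character's location and rotation to those of SelectedTarget.
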(event `self.ReceiveBeginPlay`
  (set `self.PlayerCharacter` (`self.PlayerCharacter`))
  (bind _outactors (`GameplayStatics.GetAllActorsOfClass` "/Game/Blueprints/TeleportSystem/BP_TeleportTarget.BP_TeleportTarget_C"))
  (for _array_element _outactors
    (`KismetArrayLibrary.Array_Add` (`self.TeleportTargets`) _array_element)
    (`KismetArrayLibrary.Array_Add` (`self.TargetNames`) (`KismetSystemLibrary.GetDisplayName` _array_element)))
  (bind _returnvalue (`|CreateWidget` "/Game/Blueprints/TeleportSystem/UI_TeleportMenu.UI_TeleportMenu_C" null self))
  (`KismetSystemLibrary.PrintString` "Widget Created" true true (struct :`G` 0.66 :`B` 1.0 :`A` 1.0) 15.0)
  (`UserWidget.AddToViewport` _returnvalue 0))

(event `ExecuteTeleport`
  (bind _playercharacter (`self.PlayerCharacter`))
  (bind _returnvalue (`|CreateWidget` "/Game/Blueprints/TeleportSystem/UI_FadeOverlay.UI_FadeOverlay_C"))
  (`UserWidget.AddToViewport` _returnvalue 0)
  (`/Game/Blueprints/TeleportSystem/UI_FadeOverlay.PlayFadeOut` _returnvalue)
  (`KismetSystemLibrary.Delay` 1.0)
  (`/Game/Blueprints/TeleportSystem/UI_FadeOverlay.PlayFadeIn` _returnvalue)
  (`KismetSystemLibrary.PrintString` (`/Game/Blueprints/TeleportSystem/BP_TeleportTarget.TargetName` (`self.SelectedTarget`)) true true (struct :`G` 0.66 :`B` 1.0 :`A` 1.0) 10.0)
  (if (`KismetSystemLibrary.IsValid` (`self.PlayerCharacter`))
    (`self.K2_SetActorLocation` _playercharacter (`self.K2_GetActorLocation` (`self.SelectedTarget`)) false false)
    (`self.K2_SetActorRotation` _playercharacter (`self.K2_GetActorRotation` (`self.SelectedTarget`)) false)
    (else
      (`KismetSystemLibrary.PrintString` "CharacterUndefined" true true (struct :`G` 0.66 :`B` 1.0 :`A` 1.0) 10.0))))

(fn `UserConstructionScript`)